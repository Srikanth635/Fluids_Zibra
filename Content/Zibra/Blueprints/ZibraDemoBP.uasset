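; Demo controller Blueprint for Zibra Liquid that lets the player toggle gravity, an emitter and a force field at runtime.
; BeginPlay fetches the emitter and force field components from referenced actors, sets the field to radial, creates the ZibraDemoUI widget and enables input.
; Key 1 switches between downward and weaker upward gravity; E and Q toggle the emitter and force field.
; Tick applies gravity to the liquid every frame and displays it in the widget.
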(event `self.ReceiveBeginPlay`
  (set `self.ForceField` (`self.GetComponentByClass` (`self.ForceFieldActor`) "/Script/ZibraAILiquidRuntime.ZibraLiquidForceField"))
  (`ZibraLiquidForceField.SetType` (`self.ForceField`) "EForceFieldType_Radial")
  (set `self.Emitter` (`self.GetComponentByClass` (`self.EmitterActor`) "/Script/ZibraAILiquidRuntime.ZibraLiquidEmitter"))
  (bind _returnvalue (`|CreateWidget` "/Game/Zibra/Blueprints/ZibraDemoUI.ZibraDemoUI_C"))
  (bind _output_get (set `self.ZibraDemoUI` _returnvalue))
  (`UserWidget.AddToViewport` _output_get 0)
  (`self.EnableInput` (`GameplayStatics.GetPlayerController` 0)))

(event `Key|One`
  (params (Key :type "Key Structure"))
  (:`Released`
    (set `self.DefaultGravity` (not (`self.DefaultGravity`)))))

(event `Key|E`
  (params (Key :type "Key Structure"))
  (bind _emitter (`self.Emitter`))
  (:`Released`
    (bind _output_get (set `self.EmitterEnable` (not (`self.EmitterEnable`))))
    (if _output_get
      (`ZibraLiquidEmitter.Enable` _emitter)
      (else
        (`ZibraLiquidEmitter.Disable` _emitter)))))

(event `self.ReceiveTick`
  (params (DeltaSeconds :type "Float (single-precision)"))
  (bind _liquid (`self.Liquid`))
  (if (`self.DefaultGravity`)
    (`ZibraLiquid.SetGravity` _liquid (0.0 0.0 -9.81))
    (else
      (`ZibraLiquid.SetGravity` _liquid (0.0 0.0 3.0))))
  (bind _returnvalue (`ZibraLiquid.GetGravity` _liquid))
  (`TextBlock.SetText` (`/Game/Zibra/Blueprints/ZibraDemoUI.GravityText` (`self.ZibraDemoUI`)) (`KismetTextLibrary.Conv_VectorToText` _returnvalue)))

(event `Key|Q`
  (params (Key :type "Key Structure"))
  (bind _forcefield (`self.ForceField`))
  (:`Released`
    (bind _output_get (set `self.ForceFieldEnable` (not (`self.ForceFieldEnable`))))
    (if _output_get
      (`ZibraLiquidForceField.Enable` _forcefield)
      (else
        (`ZibraLiquidForceField.Disable` _forcefield)))))

(fn `UserConstructionScript`)